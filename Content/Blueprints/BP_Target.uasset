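; BP_Target is a replicated target actor that changes to a random color after being hit.
; On Tick, the authority checks IsHit, which is set outside this graph, clears it and assigns a random CurrentColor.
; The CurrentColor OnRep creates a new dynamic material instance and sets its Color parameter.
; The construction script also creates an instance in DynamicMaterial, which the OnRep does not use.
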(event EventTick
  (params (DeltaSeconds :type Float%20%28single-precision%29))
  (Networking|SwitchHasAuthority
    (:Authority
      (if (Variables|Default|GetisHit)
        (Variables|Default|SetisHit false)
        (Variables|Default|SetCurrentColor (Math|Color|MakeColor (Math|Random|RandomFloatinRange 0.0 1.0) (Math|Random|RandomFloatinRange 0.0 1.0) (Math|Random|RandomFloatinRange 0.0 1.0)))))))

(fn ConstructionScript
  (bind _returnvalue (Rendering|Material|CreateDynamicMaterialInstance (Variables|Default|GetTarget) 0 0 :!class /Script/Engine.PrimitiveComponent))
  (Variables|Default|SetDynamicMaterial _returnvalue))

(fn OnRepCurrentColor
  (Networking|SwitchHasAuthority
    (:Authority
      _)
    (:Remote
      _))
  (bind _returnvalue (Rendering|Material|CreateDynamicMaterialInstance (Variables|Default|GetTarget) 0 0 :!class /Script/Engine.PrimitiveComponent))
  (bind _output_get (Variables|Default|SetMaterial%20Reference _returnvalue))
  (Rendering|Material|SetVectorParameterValue _output_get "Color" (Variables|Default|GetCurrentColor) :!class /Script/Engine.MaterialInstanceDynamic))