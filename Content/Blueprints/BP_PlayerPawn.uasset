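; Player pawn that adds crosshair and health bar widgets for the local player and supports a replicated body color.
; On BeginPlay, a random CurrentColor is picked only if the pawn is both locally controlled and has authority.
; Its RepNotify creates a dynamic mesh material and sets BodyColor from that color; its authority switch is empty.
; The construction script creates a separate DynamicMaterial instance that the RepNotify does not use.
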(event EventBeginPlay
  (if (Pawn|IsLocallyControlled)
    (Utilities|FlowControl|Sequence
      (:then_0
        (bind _returnvalue (UserInterface|CreateWidget "/Game/UI/WBP_Crosshair.WBP_Crosshair_C"))
        (UserInterface|Viewport|AddtoViewport _returnvalue 0))
      (:then_1
        (bind _returnvalue_2 (UserInterface|CreateWidget "/Game/UI/WBP_HealthBar.WBP_HealthBar_C"))
        (UserInterface|Viewport|AddtoViewport _returnvalue_2 0))
      (:then_2
        (Networking|SwitchHasAuthority
          (:Authority
            (Variables|Default|SetCurrentColor (Math|Color|MakeColor (Math|Random|RandomFloatinRange 0.0 1.0) (Math|Random|RandomFloatinRange 0.0 1.0) (Math|Random|RandomFloatinRange 0.0 1.0)))))))))

(fn ConstructionScript
  (bind _returnvalue (Rendering|Material|CreateDynamicMaterialInstance (Variables|Character|GetMesh) 0 0 :!class /Script/Engine.PrimitiveComponent))
  (Variables|Default|SetDynamicMaterial _returnvalue))

(fn OnRepCurrentColor
  (Networking|SwitchHasAuthority
    (:Authority
      _)
    (:Remote
      _))
  (bind _returnvalue (Rendering|Material|CreateDynamicMaterialInstance (Variables|Character|GetMesh) 0 0 :!class /Script/Engine.PrimitiveComponent))
  (bind _output_get (Variables|Default|SetMaterial%20Reference _returnvalue))
  (Rendering|Material|SetVectorParameterValue _output_get "BodyColor" (Variables|Default|GetCurrentColor) :!class /Script/Engine.MaterialInstanceDynamic))